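; BP_Marine is a player-controlled marine pawn that moves along its own forward and right axes and aims by setting controller yaw.
; Every tick it updates aim from the thumbstick or mouse, chosen by whether the last key pressed was a gamepad key.
; Both inputs use dead zones: stick angle sets yaw directly, while mouse aim smoothly interpolates toward the direction of mouse velocity rather than cursor position.
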(event `self.ReceiveTick`
  (params (DeltaSeconds :type "Float (single-precision)"))
  (`self.UpdatePlayerAim`))

(event `InputAxis|Thumbstick AimUp`
  (params (AxisValue :type "Float (single-precision)"))
  ;[1 1 1] Used For Testing
)

(event `InputAxis|MoveForward`
  (params (AxisValue :type "Float (single-precision)"))
  (`self.AddMovementInput` (`self.GetActorForwardVector`) AxisValue))

(event `InputAxis|Thumbstick AimRight`
  (params (AxisValue :type "Float (single-precision)"))
  ;[1 1 1] Used For Testing
)

(event `InputAxis|MoveRight`
  (params (AxisValue :type "Float (single-precision)"))
  (`self.AddMovementInput` (`self.GetActorRightVector`) AxisValue))

(event `Key|AnyKey`
  (params (Key :type "Key Structure"))
  (:`Pressed`
    (set `self.IsGamepadActive` (`KismetInputLibrary.Key_IsGamepadKey` Key))))

(fn `Get Mouse Aim Direction`
  (returns (ReturnValue :type "Rotator Structure"))
  (bind (_return_value_x _return_value_y) (`KismetMathLibrary.BreakVector2D` (`self.GetMouseVelocity`)))
  (return (`KismetMathLibrary.RInterpTo` (`Controller.GetControlRotation` (`GameplayStatics.GetPlayerController` 0)) (`KismetMathLibrary.MakeRotator` 0.0 0.0 (`KismetMathLibrary.DegAtan2` _return_value_x _return_value_y)) (`GameplayStatics.GetWorldDeltaSeconds`) (`self.MouseSmoothingStrength`))))

(fn `GetMouseVelocity`
  (returns (`Return Value` :type "Vector2D Structure"))
  (bind (_deltax _deltay) (`PlayerController.GetInputMouseDelta` (`GameplayStatics.GetPlayerController` 0)))
  (return (/ (`KismetMathLibrary.MakeVector2D` _deltax _deltay) (`GameplayStatics.GetWorldDeltaSeconds`))))

(fn `GetThumbstickAimDirection`
  (returns (ReturnValue :type "Rotator Structure"))
  (return (`KismetMathLibrary.MakeRotator` 0.0 0.0 (`KismetMathLibrary.DegAtan2` (`self.GetInputAxisValue`) (`self.GetInputAxisValue`)))))

(fn `IsMouseAboveDeadZone`
  (returns (ReturnValue :type Boolean))
  (return (> (`KismetMathLibrary.VSize2D` (`self.GetMouseVelocity`)) (`self.MouseDeadZone`))))

(fn `IsThumbstickAboveDeadZone`
  (returns (ReturnValue :type Boolean))
  (return (> (`KismetMathLibrary.VSize2D` (`KismetMathLibrary.MakeVector2D` (`self.GetInputAxisValue`) (`self.GetInputAxisValue`))) (`self.ThumbstickDeadZone`))))

(fn `UpdateMouseAim`
  (if (`self.IsMouseAboveDeadZone`)
    (`Controller.SetControlRotation` (`GameplayStatics.GetPlayerController` 0) (`self.Get Mouse Aim Direction`))))

(fn `UpdatePlayerAim`
  (if (`self.IsGamepadActive`)
    (`self.UpdateThumbstickAim`)
    (else
      (`self.UpdateMouseAim`))))

(fn `UpdateThumbstickAim`
  (if (`self.IsThumbstickAboveDeadZone`)
    (`Controller.SetControlRotation` (`GameplayStatics.GetPlayerController` 0) (`self.GetThumbstickAimDirection`))))

(fn `UserConstructionScript`)